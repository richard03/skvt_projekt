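; BP_WallSconce is a wall sconce light with configurable on state, brightness, color and cone angles.
; The construction script applies these settings to the SconceLight component.
; ToggleLight flips IsOn, and its RepNotify function updates the light's visibility to keep the on/off state in sync over the network.
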(fn ConstructionScript
  (bind _sconcelight (Variables|Default|GetSconceLight))
  (Rendering|SetVisibility _sconcelight (Variables|Light|GetisOn) false)
  (Rendering|Components|Light|SetIntensity _sconcelight (Variables|Light|GetBrightness))
  (Rendering|Components|Light|SetLightColor _sconcelight (Variables|Light|GetColor) true)
  (Rendering|Lighting|SetInnerConeAngle _sconcelight (Variables|Light|GetInner%20Cone%20Angle))
  (Rendering|Lighting|SetOuterConeAngle _sconcelight (Variables|Light|GetOuter%20Cone%20Angle)))

(fn ToggleLight
  (Variables|Light|SetisOn (not (Variables|Light|GetisOn))))

(fn OnRepIson
  (Rendering|SetVisibility (Variables|Default|GetSconceLight) (Variables|Light|GetisOn) false))